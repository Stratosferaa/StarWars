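; Pressure door actor that can swing open automatically when the player enters its trigger box and close after they leave.
; A DoorOpening timeline drives door yaw and lever pitch, playing forward on entry and reversing on exit.
; DoOnce gates and a DoorOpen flag guard retriggering, while door collision is disabled during movement.
; The construction script poses door and lever from a clamped DoorRotation value.
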(event OnComponentBeginOverlap(TriggerBox)
  (params (OverlappedComponent :type Primitive%20Component%20Object%20Reference) (OtherActor :type Actor%20Object%20Reference) (OtherComp :type Primitive%20Component%20Object%20Reference) (OtherBodyIndex :type Integer) (bFromSweep :type Boolean) (SweepResult :type Hit%20Result%20Structure%20%28by%20ref%29))
  ;[1 1 1] Automatic Door Opening Mechanism
  (if (Math|Boolean|ANDBoolean (Variables|Default|GetAutomaticDoor) (== (Game|Player|GetPlayerPawn 0) OtherActor) (not (Variables|Default|GetDoorOpen)))
    (Utilities|FlowControl|DoOnce false :!label _label
      (:Completed
        (Collision|SetCollisionEnabled (Variables|Default|GetSM_Pressure_Door) "NoCollision")
        (bind (_direction _dooropening _doorhandleopening) (Timeline|DoorOpening PlayFromStart)
          (:Update
            (Transformation|SetRelativeRotation (Variables|Default|GetSM_Pressure_Door) (Math|Rotator|MakeRotator 0.0 0.0 _dooropening) false false)
            (Transformation|SetRelativeRotation (Variables|Default|GetSM_Pressure_Door_Lever) (Math|Rotator|MakeRotator 0.0 _doorhandleopening 0.0) false false))
          (:Finished
            (if (Utilities|Enum|Equal(Enum) _direction "Forward")
              (Variables|Default|SetDoorOpen true)
              (else
                (Variables|Default|SetDoorOpen false)))
            (Collision|SetCollisionEnabled (Variables|Default|GetSM_Pressure_Door) "QueryAndPhysics")
            (Utilities|FlowControl|Sequence
              (:then_0
                (goto _label Reset))
              (:then_1
                (Utilities|FlowControl|DoOnce false) ; enters at Reset
              ))))))))

(event OnComponentEndOverlap(TriggerBox)
  (params (OverlappedComponent :type Primitive%20Component%20Object%20Reference) (OtherActor :type Actor%20Object%20Reference) (OtherComp :type Primitive%20Component%20Object%20Reference) (OtherBodyIndex :type Integer))
  ;[1 1 1] Automatic Door Opening Mechanism
  (if (and (Variables|Default|GetDoorOpen) (== (Game|Player|GetPlayerPawn 0) OtherActor))
    (Utilities|FlowControl|DoOnce false :!label _label
      (:Completed
        (Collision|SetCollisionEnabled (Variables|Default|GetSM_Pressure_Door) "NoCollision")
        (bind (_direction _dooropening _doorhandleopening) (Timeline|DoorOpening ReverseFromEnd)
          (:Update
            (Transformation|SetRelativeRotation (Variables|Default|GetSM_Pressure_Door) (Math|Rotator|MakeRotator 0.0 0.0 _dooropening) false false)
            (Transformation|SetRelativeRotation (Variables|Default|GetSM_Pressure_Door_Lever) (Math|Rotator|MakeRotator 0.0 _doorhandleopening 0.0) false false))
          (:Finished
            (if (Utilities|Enum|Equal(Enum) _direction "Forward")
              (Variables|Default|SetDoorOpen true)
              (else
                (Variables|Default|SetDoorOpen false)))
            (Collision|SetCollisionEnabled (Variables|Default|GetSM_Pressure_Door) "QueryAndPhysics")
            (Utilities|FlowControl|Sequence
              (:then_0
                (Utilities|FlowControl|DoOnce false) ; enters at Reset
              )
              (:then_1
                (goto _label Reset)))))))))

(event EventBeginPlay)

(event Collision|EventActorBeginOverlap
  (params (OtherActor :type Actor%20Object%20Reference)))

(event EventTick
  (params (DeltaSeconds :type Float%20%28single-precision%29)))

(fn ConstructionScript
  (bind _sm_pressure_door_lever (Variables|Default|GetSM_Pressure_Door_Lever))
  ;[1 1 1] Open/Close Door and Rotate Lever based on that
  (Transformation|SetRelativeRotation (Variables|Default|GetSM_Pressure_Door) (Math|Rotator|MakeRotator 0.0 0.0 (Math|Float|Clamp(Float) (Variables|Default|GetDoorRotation) -1.2e+02 1.2e+02)) false false)
  (if (>= (Variables|Default|GetDoorRotation) 1.0)
    (Transformation|SetRelativeRotation _sm_pressure_door_lever "70.000000, 0, 0" false false)
    (else
      (Transformation|SetRelativeRotation _sm_pressure_door_lever "0, 0, 0" false false))))
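; BP_Module_Center_End is a planet-surface building module whose interior lights power up when the player enters and power down when they leave.
; BeginPlay creates a dynamic material on the interior mesh and starts the light and emissive glow at zero.
; Capsule overlaps play a timeline forward or in reverse, driving light intensity and emissive multiplier.
; An Activated flag and two DoOnce gates, reset when the timeline finishes, prevent retriggering mid-transition.
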(event OnComponentBeginOverlap(Capsule)
  (params (OverlappedComponent :type Primitive%20Component%20Object%20Reference) (OtherActor :type Actor%20Object%20Reference) (OtherComp :type Primitive%20Component%20Object%20Reference) (OtherBodyIndex :type Integer) (bFromSweep :type Boolean) (SweepResult :type Hit%20Result%20Structure%20%28by%20ref%29))
  ;[1 1 1] Module Activation
  (if (and (== (Game|Player|GetPlayerPawn 0) OtherActor) (not (Variables|Default|GetActivated)))
    (Utilities|FlowControl|DoOnce false :!label _label
      (:Completed
        (bind (_direction _lightsintensity _emissiveintensity) (Timeline|Timeline_0 PlayFromStart)
          (:Update
            (Rendering|Components|Light|SetIntensity (Variables|Default|GetInteriorLight) _lightsintensity)
            (Rendering|Material|SetScalarParameterValue (Variables|Default|GetMatInst) "LightingMultiplier" _emissiveintensity :!class /Script/Engine.MaterialInstanceDynamic))
          (:Finished
            (if (Utilities|Enum|Equal(Enum) _direction "Forward")
              (Variables|Default|SetActivated true)
              (else
                (Variables|Default|SetActivated false)))
            (Utilities|FlowControl|Sequence
              (:then_0
                (goto _label Reset))
              (:then_1
                (Utilities|FlowControl|DoOnce false) ; enters at Reset
              ))))))))

(event OnComponentEndOverlap(Capsule)
  (params (OverlappedComponent :type Primitive%20Component%20Object%20Reference) (OtherActor :type Actor%20Object%20Reference) (OtherComp :type Primitive%20Component%20Object%20Reference) (OtherBodyIndex :type Integer))
  ;[1 1 1] Module Activation
  (if (and (Variables|Default|GetActivated) (== (Game|Player|GetPlayerPawn 0) OtherActor))
    (Utilities|FlowControl|DoOnce false :!label _label
      (:Completed
        (bind (_direction _lightsintensity _emissiveintensity) (Timeline|Timeline_0 ReverseFromEnd)
          (:Update
            (Rendering|Components|Light|SetIntensity (Variables|Default|GetInteriorLight) _lightsintensity)
            (Rendering|Material|SetScalarParameterValue (Variables|Default|GetMatInst) "LightingMultiplier" _emissiveintensity :!class /Script/Engine.MaterialInstanceDynamic))
          (:Finished
            (if (Utilities|Enum|Equal(Enum) _direction "Forward")
              (Variables|Default|SetActivated true)
              (else
                (Variables|Default|SetActivated false)))
            (Utilities|FlowControl|Sequence
              (:then_0
                (Utilities|FlowControl|DoOnce false) ; enters at Reset
              )
              (:then_1
                (goto _label Reset)))))))))

(event EventBeginPlay
  (bind _sm_module_center_int (Variables|Default|GetSM_Module_Center_Int))
  ;[1 1 1] Create Dynamic Material Instance and Set Default Values
  (bind _returnvalue (Rendering|Material|CreateDynamicMaterialInstance _sm_module_center_int 1 (Rendering|Material|GetMaterial _sm_module_center_int 1) "None" :!class /Script/Engine.PrimitiveComponent))
  (bind _output_get (Variables|Default|SetMatInst _returnvalue))
  (Rendering|Material|SetScalarParameterValue _output_get "LightingMultiplier" 0.0 :!class /Script/Engine.MaterialInstanceDynamic)
  (Rendering|Components|Light|SetIntensity (Variables|Default|GetInteriorLight) 0.0))

(event Collision|EventActorBeginOverlap
  (params (OtherActor :type Actor%20Object%20Reference)))

(event EventTick
  (params (DeltaSeconds :type Float%20%28single-precision%29)))

(fn ConstructionScript)
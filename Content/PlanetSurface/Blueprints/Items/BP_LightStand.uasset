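; BP_LightStand is a placeable light stand prop whose lit state and color are configurable.
; Its construction script creates a dynamic material instance on the stand mesh and uses the LightOn flag to set emissive strength.
; When on, the emissive and light component take LightColor; when off, the light and cone mesh are hidden.
; The event graph holds no active logic.
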(event EventBeginPlay)

(event Collision|EventActorBeginOverlap
  (params (OtherActor :type Actor%20Object%20Reference)))

(event EventTick
  (params (DeltaSeconds :type Float%20%28single-precision%29)))

(fn ConstructionScript
  (bind _sm_light_stand (Variables|Default|GetSM_Light_Stand))
  (bind _light (Variables|Default|GetLight))
  ;[1 1 1] Toggle light and set values
  (bind _returnvalue (Rendering|Material|CreateDynamicMaterialInstance _sm_light_stand 0 (Rendering|Material|GetMaterial _sm_light_stand 0) "None" :!class /Script/Engine.PrimitiveComponent))
  (Variables|Default|SetMaterialInstance _returnvalue)
  (if (Variables|Default|GetLightOn)
    (Rendering|Material|SetScalarParameterValue (Variables|Default|GetMaterialInstance) "EmissiveMultiplier" 6.0 :!class /Script/Engine.MaterialInstanceDynamic)
    (Rendering|Material|SetVectorParameterValue (Variables|Default|GetMaterialInstance) "EmissiveColor" (Variables|Default|GetLightColor) :!class /Script/Engine.MaterialInstanceDynamic)
    (Rendering|SetVisibility _light true false)
    (Rendering|Components|Light|SetLightColor _light (Variables|Default|GetLightColor) true)
    (else
      (Rendering|Material|SetScalarParameterValue (Variables|Default|GetMaterialInstance) "EmissiveMultiplier" 0.0 :!class /Script/Engine.MaterialInstanceDynamic)
      (Rendering|SetVisibility _light false false))))
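; BP_Aerophonic is a placeable aerophonic prop for the planet surface, with a power state and selectable foliage growth stage.
; The construction script creates a dynamic material instance, and PowerOn toggles its emissive glow and the light's visibility.
; FoliageStages picks one of three static meshes for no, medium or high foliage.
; Everything is set at construction; the event graph has no active logic.
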(event EventBeginPlay)

(event Collision|EventActorBeginOverlap
  (params (OtherActor :type Actor%20Object%20Reference)))

(event EventTick
  (params (DeltaSeconds :type Float%20%28single-precision%29)))

(fn ConstructionScript
  (bind _sm_aerophonic (Variables|Default|GetSM_Aerophonic))
  (bind _light (Variables|Default|GetLight))
  ;[1 1 1] Power Control
  (bind _returnvalue (Rendering|Material|CreateDynamicMaterialInstance _sm_aerophonic 0 (Rendering|Material|GetMaterial _sm_aerophonic 0) "None" :!class /Script/Engine.PrimitiveComponent))
  (Variables|Default|SetMaterialInstance _returnvalue)
  (if (Variables|Default|GetPowerOn)
    (Rendering|Material|SetScalarParameterValue (Variables|Default|GetMaterialInstance) "EmissiveMultiplier" 6.0 :!class /Script/Engine.MaterialInstanceDynamic)
    (Rendering|SetVisibility _light true false)
    (else
      (Rendering|Material|SetScalarParameterValue (Variables|Default|GetMaterialInstance) "EmissiveMultiplier" 0.0 :!class /Script/Engine.MaterialInstanceDynamic)
      (Rendering|SetVisibility _light false false)))
  ;[1 1 1] Foliage Stages
  (Components|StaticMesh|SetStaticMesh (Variables|Default|GetSM_Aerophonic) (Utilities|Select :Index (Variables|Default|GetFoliageStages) :NewEnumerator0 "/Game/PlanetSurface/Models/Structure/Devices/SM_Aerophonic1.SM_Aerophonic1" :NewEnumerator1 "/Game/PlanetSurface/Models/Structure/Devices/SM_Aerophonic2.SM_Aerophonic2" :NewEnumerator2 "/Game/PlanetSurface/Models/Structure/Devices/SM_Aerophonic3.SM_Aerophonic3")))
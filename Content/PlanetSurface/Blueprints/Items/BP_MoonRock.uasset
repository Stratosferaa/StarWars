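; Moon rock item for the planet surface: a randomized small rock that can be picked up and dropped.
; The construction script picks a small rock mesh at random and randomizes its scale and mass.
; Pickup disables physics and pawn blocking and attaches the mesh to the given component; Drop restores both and detaches.
; After a startup delay, hits with enough relative velocity spawn tire-dust particles, throttled by a DoOnce with delayed reset.
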(event OnComponentHit(StaticMesh)
  (params (HitComponent :type Primitive%20Component%20Object%20Reference) (OtherActor :type Actor%20Object%20Reference) (OtherComp :type Primitive%20Component%20Object%20Reference) (NormalImpulse :type Vector :default "0, 0, 0") (Hit :type Hit%20Result%20Structure%20%28by%20ref%29))
  (bind (_bblockinghit _binitialoverlap _time _distance _location _impactpoint _normal _impactnormal _physmat _hitactor _hitcomponent) (Collision|BreakHitResult Hit))
  (if (Variables|Default|GetAllowEffects)
    ;[1 1 1] Impulse large enough?
    (if (> (Math|Vector|VectorLength (- (Transformation|GetComponentVelocity HitComponent) (Transformation|GetComponentVelocity _hitcomponent))) 7e+01)
      ;[1 1 1] Add Effect
      (Utilities|FlowControl|DoOnce false :!label _label
        (:Completed
          (Effects|SpawnEmitteratLocation "/Game/PlanetSurface/Vehicle/Effects/PS_Effect_TireDust.PS_Effect_TireDust" _impactpoint "0, 0, 0" "1.000000,1.000000,1.000000" false)
          (Utilities|FlowControl|Delay 0.4)
          (goto _label Reset))))))

(event Collision|EventActorBeginOverlap
  (params (OtherActor :type Actor%20Object%20Reference)))

(event EventTick
  (params (DeltaSeconds :type Float%20%28single-precision%29)))

(event EventBeginPlay
  (Utilities|FlowControl|Delay 5.0)
  (Variables|Default|SetAllowEffects true))

(event EventPickup
  (params (AttachTo :type Scene%20Component%20Object%20Reference))
  (bind _staticmesh (Variables|Default|GetStaticMesh))
  ;[1 1 1] Pick Up
  (Physics|SetSimulatePhysics _staticmesh false)
  (Collision|SetCollisionResponsetoChannel _staticmesh "ECC_Pawn" "ECR_Ignore")
  (Transformation|AttachComponentToComponent _staticmesh AttachTo "None" "SnapToTarget" "KeepWorld" "KeepWorld" false))

(event EventDrop
  (bind _staticmesh (Variables|Default|GetStaticMesh))
  ;[1 1 1] Drop
  (Physics|SetSimulatePhysics _staticmesh true)
  (Collision|SetCollisionResponsetoChannel _staticmesh "ECC_Pawn" "ECR_Block")
  (Transformation|DetachFromActor (Components|GetOwner _staticmesh) "KeepWorld" "KeepWorld" "KeepWorld"))

(fn ConstructionScript
  (bind _staticmesh (Variables|Default|GetStaticMesh))
  ;[1 1 1] Create Random Small Rock
  (Components|StaticMesh|SetStaticMesh (Variables|Default|GetStaticMesh) (Utilities|Select :Index (Math|Random|RandomInteger 4) :Option%200 "/Game/PlanetSurface/Models/Nature/Rocks/SM_Rock_Small_1.SM_Rock_Small_1" :Option%201 "/Game/PlanetSurface/Models/Nature/Rocks/SM_Rock_Small_2.SM_Rock_Small_2" :Option%202 "/Game/PlanetSurface/Models/Nature/Rocks/SM_Rock_Small_3.SM_Rock_Small_3" :Option%203 "/Game/PlanetSurface/Models/Nature/Rocks/SM_Rock_Small_4.SM_Rock_Small_4" :Option%204 "/Game/PlanetSurface/Models/Nature/Rocks/SM_Rock_Small_5.SM_Rock_Small_5"))
  (Rendering|Material|SetMaterial _staticmesh 0 "/Game/PlanetSurface/Materials/Nature/Rocks/MI_Rock_Small_Pickable.MI_Rock_Small_Pickable")
  (Transformation|SetWorldScale3D _staticmesh (* "1.000000,1.000000,1.000000" (Math|Random|RandomFloatinRange 0.1 0.5)))
  (Class|PrimitiveComponent|SetMassOverrideinKg _staticmesh "None" (Math|Random|RandomFloatinRange 1e+01 2e+01) true))
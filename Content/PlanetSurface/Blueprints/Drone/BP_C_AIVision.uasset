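; Drone AI vision component that scans and marks actors in the camera's line of sight.
; Tick traces forward, ignoring landscape, foliage and marked actors, then highlights the hit via custom depth for an object-tracking post process and zooms in.
; A ScanningTime timer marks the focused actor with a stencil value chosen by collision type, shown in the AI Vision widget.
; A looping timer flushes temporary highlights; a separate function clears marks and compass.
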(event Custom|Flushing
  ;[1 1 1] Flush HightlightedActors Array
  (CallFunction|FlushHightlightedActors))

(event Custom|InitializeAIVision
  ;[1 1 1] Event Begin
  ;[1 1 1] Add AI Vision Widget to Viewport and Give Reference
  (Viewport|RemoveAllWidgets)
  (bind _returnvalue (UserInterface|CreateWidget "/Game/PlanetSurface/Blueprints/Drone/UI_AIVision.UI_AIVision_C"))
  (bind _output_get (Variables|References|SetAIVisionUIRef _returnvalue))
  (Variables|/Game/PlanetSurface/Blueprints/Drone/UI_AIVision.UI_AIVision_C|SetAIVisionRef _output_get self)
  (UserInterface|Viewport|AddtoViewport _output_get 0)
  ;[1 1 1] Add Object Tracking Post Process Effect
  (Variables|/Script/Engine.CameraComponent|SetPostProcessSettings (Variables|References|GetCamera) (Utilities|Struct|MakePostProcessSettings (Utilities|Struct|MakeWeightedBlendables (Utilities|Array|MakeArray (Utilities|Struct|MakeWeightedBlendable 1.0 (Variables|Scanning|GetObjectTrackingPostProcess))))))
  (Utilities|Time|SetTimerbyEvent (delegate Custom|Flushing) 2.0 true)
  ;[1 1 1] Set Tick enabled after short delay to avoid issues
  (Utilities|FlowControl|Delay 1.0)
  (Components|Tick|SetComponentTickEnabled true))

(event EventBeginPlay)

(event EventTick
  (params (DeltaSeconds :type Float%20%28single-precision%29))
  (bind _camera (Variables|References|GetCamera))
  (bind _maxzoomfov (Variables|Scanning|GetMaxZoomFOV))
  (bind _defaultfov (Variables|Scanning|GetDefaultFOV))
  (bind _aivisionuiref (Variables|References|GetAIVisionUIRef))
  (bind _camera_2 (Variables|References|GetCamera))
  (bind _returnvalue (Transformation|GetWorldTransform _camera_2))
  (bind _fieldofview (Variables|/Script/Engine.CameraComponent|GetFieldOfView _camera))
  (bind _fieldofview_2 (Variables|/Script/Engine.CameraComponent|GetFieldOfView _camera))
  (bind _returnvalue_2 (Math|Interpolation|FInterpTo _fieldofview _defaultfov DeltaSeconds 5.0))
  (bind _returnvalue_3 (Math|Interpolation|FInterpTo _fieldofview_2 _maxzoomfov DeltaSeconds 1.0))
  ;[1 1 1] Event Tick
  ;[1 1 1] Line Trace
  (bind _outhit (Collision|LineTraceByChannel (.location _returnvalue) (+ (.location _returnvalue) (* (Math|Vector|GetForwardVector (.rotation _returnvalue)) (Variables|Scanning|GetScanningDistance))) "TraceTypeQuery1" true 0 "None" true "(R=1.000000,G=0.000000,B=0.000000,A=1.000000)" "(R=0.000000,G=1.000000,B=0.000000,A=1.000000)" 1.0))
  ;[1 1 1] Check if Blocking hit and not landscape, InstFol or MarkedActor
  (if (and (not (Math|Boolean|ORBoolean (== (Utilities|GetClass (.HitActor (Collision|BreakHitResult _outhit))) "/Script/Landscape.Landscape") (== (Utilities|GetClass (.HitActor (Collision|BreakHitResult _outhit))) "/Script/Foliage.InstancedFoliageActor") (Utilities|Array|ContainsItem (Variables|Scanning|GetMarkedActors) (.HitActor (Collision|BreakHitResult _outhit))))) (.bBlockingHit (Collision|BreakHitResult _outhit)))
    ;[1 1 1] First Hightlighting
    (bind _output_get (Variables|Scanning|SetFocalActor (.HitActor (Collision|BreakHitResult _outhit))))
    (Variables|/Game/PlanetSurface/Blueprints/Drone/UI_AIVision.UI_AIVision_C|SetFocusActor (Variables|References|GetAIVisionUIRef) _output_get)
    (CallFunction|ActorHightlighting)
    ;[1 1 1] Scanning
    (Utilities|IsValid (Variables|Scanning|GetFocalActor)
      (:Is%20Valid
        (Camera|SetFieldOfView _camera _returnvalue_3)
        (bind _output_get_2 (Variables|Scanning|SetCurrentFOV _returnvalue_3))
        (Default|Scanning _aivisionuiref _output_get_2 true)
        (Utilities|FlowControl|DoOnce false :!label _label
          (:Completed
            ;;[1 1 1] Mark Actor when ScanningTime is met
            (Utilities|Time|SetTimerbyFunctionName 0 "ActorMarking" (Variables|Scanning|GetScanningTime) true)))))
    (else
      (Variables|Scanning|SetFocalActor 0)
      (Camera|SetFieldOfView _camera _returnvalue_2)
      (bind _output_get_3 (Variables|Scanning|SetCurrentFOV _returnvalue_2))
      (Default|Scanning _aivisionuiref _output_get_3 false)
      (goto _label Reset))))

(fn ActorHightlighting
  (bind _focalactor (Variables|Scanning|GetFocalActor))
  (for _array_element (Actor|GetComponentsByClass _focalactor "/Script/Engine.PrimitiveComponent")
    ;[1 1 1] Set FocalActor custom depth values
    (Rendering|SetRenderCustomDepth _array_element true)
    (Rendering|SetCustomDepthStencilValue _array_element 1))
  ;[1 1 1] Add to HightlightedActors Array
  (Utilities|Array|Add (Variables|Scanning|GetHighlightedActors) _focalactor))

(fn ActorMarking
  (bind _focalactor (Variables|Scanning|GetFocalActor))
  (Utilities|IsValid _focalactor
    (:Is%20Valid
      (for _array_element (Actor|GetComponentsByClass _focalactor "/Script/Engine.PrimitiveComponent")
        ;[1 1 1] Set FocalActor custom depth values
        (Rendering|SetRenderCustomDepth _array_element true)
        (Rendering|SetCustomDepthStencilValue _array_element (Utilities|Select :Index (Collision|GetCollisionObjectType _array_element) :ECC_WorldStatic 2 :ECC_WorldDynamic 2 :ECC_Pawn 2 :ECC_Visibility 2 :ECC_Camera 2 :ECC_PhysicsBody 4 :ECC_Vehicle 3 :ECC_Destructible 2))
        ;[1 1 1] Add UI Marking
        (Utilities|FlowControl|DoOnce false
          (:Completed
            (Default|Marking (Variables|References|GetAIVisionUIRef) (Utilities|Select :Index (Collision|GetCollisionObjectType _array_element) :ECC_WorldStatic 2 :ECC_WorldDynamic 2 :ECC_Pawn 2 :ECC_Visibility 2 :ECC_Camera 2 :ECC_PhysicsBody 4 :ECC_Vehicle 3 :ECC_Destructible 2)))))
      ;[1 1 1] Remove from HightlightedActors Array and add to MarkedActors Arra
      (Utilities|Array|RemoveItem (Variables|Scanning|GetHighlightedActors) _focalactor)
      (Utilities|Array|Add (Variables|Scanning|GetMarkedActors) _focalactor)
      (Utilities|FlowControl|DoOnce false) ; enters at Reset
    )))

(fn FlushHightlightedActors
  ;[1 1 1] Flush Hightlighted Actors
  (for _array_element (Variables|Scanning|GetHighlightedActors)
    (for _array_element_2 (Actor|GetComponentsByClass _array_element "/Script/Engine.PrimitiveComponent")
      (Rendering|SetRenderCustomDepth _array_element_2 false)))
  (Utilities|Array|Clear (Variables|Scanning|GetHighlightedActors)))

(fn FlushMarkedActors
  ;[1 1 1] Flush Marked Actors
  (for _array_element (Variables|Scanning|GetMarkedActors)
    (for _array_element_2 (Actor|GetComponentsByClass _array_element "/Script/Engine.PrimitiveComponent")
      (Rendering|SetRenderCustomDepth _array_element_2 false)))
  (Utilities|Array|Clear (Variables|Scanning|GetMarkedActors))
  (Default|ClearCompass (Variables|References|GetAIVisionUIRef)))
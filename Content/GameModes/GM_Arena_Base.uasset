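; GM_Arena_Base is an arena game mode that spawns and assigns a PP_TestCube pawn to each joining player.
; HandleStartingNewPlayer appends the new controller to PlayerList and uses the returned index to pick a PlayerStart from GetAllActorsOfClass.
; It always spawns the cube at that start's transform with the start as owner, stores it in PlayerPawn, and possesses it with that controller.
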(event EventBeginPlay)

(event EventTick
  (params (DeltaSeconds :type Float%20%28single-precision%29)))

(event EventHandleStartingNewPlayer
  (params (NewPlayer :type Player%20Controller%20Object%20Reference))
  (bind _returnvalue (Utilities|Array|Add (Variables|Default|GetPlayer%20List) NewPlayer))
  (bind _outactors (Actor|GetAllActorsOfClass "/Script/Engine.PlayerStart"))
  (bind _returnvalue_2 (Game|SpawnActorfromClass "/Game/Characters/Pilot/Blueprints/PP_TestCube.PP_TestCube_C" (Transformation|GetActorTransform (Utilities|Array|Get(acopy) _outactors _returnvalue)) "AlwaysSpawn" "MultiplyWithRoot" (Utilities|Array|Get(acopy) _outactors _returnvalue) 0))
  (Variables|Default|SetPlayer%20Pawn _returnvalue_2)
  (Pawn|Possess (Utilities|Array|Get(acopy) (Variables|Default|GetPlayer%20List) _returnvalue) (Variables|Default|GetPlayer%20Pawn)))

(fn ConstructionScript)
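; Actor component that network-syncs the location, rotation and physics velocity of its owner's static mesh, with optional authority-only sending.
; Tick, throttled by update frequency, checks change thresholds and sends optionally integer-truncated values, though rotation passes only when nearly equal to the last sent.
; OnReps apply velocity directly and optionally interpolate transforms, snapping location beyond a maximum error.
; A server-to-multicast teleport force-syncs all three.
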(event Custom|UpdateVel
  (params (ComponentVel :type Vector))
  (Variables|Default|SetComponentVel ComponentVel))

(event Custom|UpdateVelRot
  (params (ComponentVel :type Vector) (ComponentRot :type Rotator))
  (Variables|Default|SetComponentRot ComponentRot)
  (Variables|Default|SetComponentVel ComponentVel))

(event Custom|UpdateLocVel
  (params (ComponentVel :type Vector) (ComponentLoc :type Vector))
  (Variables|Default|SetComponentVel ComponentVel)
  (Variables|Default|SetComponentLoc ComponentLoc))

(event Custom|UpdateLocVelRot
  (params (ComponentVel :type Vector) (ComponentLoc :type Vector) (ComponentRot :type Rotator))
  (Variables|Default|SetComponentRot ComponentRot)
  (Variables|Default|SetComponentVel ComponentVel)
  (Variables|Default|SetComponentLoc ComponentLoc))

(event Custom|UpdateLocRot
  (params (ComponentLoc :type Vector) (ComponentRot :type Rotator))
  (Variables|Default|SetComponentRot ComponentRot)
  (Variables|Default|SetComponentLoc ComponentLoc))

(event Custom|UpdateLoc
  (params (ComponentLoc :type Vector))
  (Variables|Default|SetComponentLoc ComponentLoc))

(event Custom|Teleport
  (CallFunction|ServerTeleport (Variables|Default|GetComponentToSync)))

(event Custom|Server_Teleport
  (params (Target :type Primitive%20Component%20Object%20Reference))
  (bind _componenttosync (Variables|Default|GetComponentToSync))
  (CallFunction|MulticastTeleport (Transformation|GetWorldLocation _componenttosync) Target (Transformation|GetWorldRotation _componenttosync) (Transformation|GetComponentVelocity _componenttosync)))

(event Custom|Multicast_Teleport
  (params (NewLocation :type Vector) (Target :type Primitive%20Component%20Object%20Reference) (NewRotation :type Rotator) (NewVel :type Vector))
  (Transformation|SetWorldLocation Target NewLocation false true)
  (Transformation|SetWorldRotation Target NewRotation false false)
  (Class|PrimitiveComponent|SetAllPhysicsLinearVelocity Target NewVel false))

(event Custom|UpdateRot
  (params (ComponentRot :type Rotator))
  (Variables|Default|SetComponentRot ComponentRot))

(event EventBeginPlay
  (bind _updatefrequency (Variables|Default|GetUpdateFrequency))
  (Variables|Default|SetComponentToSync (Actor|GetComponentbyClass (Components|GetOwner) "/Script/Engine.StaticMeshComponent"))
  (if (not (== _updatefrequency 0))
    (Class|ActorComponent|SetComponentTickInterval (/ 1.0 (Math|Conversions|ToFloat(Integer) _updatefrequency)))))

(event EventTick
  (params (DeltaSeconds :type Float%20%28single-precision%29))
  (bind (_loc _vel _rot) (Utilities|Rep))
  (bind (_loc_2 _vel_2) (Utilities|Rep))
  (bind (_loc_3 _vel_3 _rot_2) (Utilities|Rep))
  (bind (_loc_4 _vel_4 _rot_3) (Utilities|Rep))
  (if (Variables|Options|GetAuthorityRepOnly)
    (if (Ability|HasAuthority (Components|GetOwner))
      (Utilities|IsValid (Variables|Default|GetComponentToSync) :!label _label
        (:Is%20Valid
          (if (Variables|Options|GetEnabled)
            (CallFunction|Threashold)
            (if (Math|Boolean|ANDBoolean (Variables|Options|GetSync%20Location) (Variables|Options|GetSync%20Velocity) (Variables|Options|GetSync%20Rotation) (Variables|Default|GetShouldSendLoc) (Variables|Default|GetShouldSendVel) (Variables|Default|GetShouldSendRot))
              (CallFunction|UpdateLocVelRot _vel _loc _rot)
              (elif (Math|Boolean|ANDBoolean (Variables|Options|GetSync%20Location) (Variables|Options|GetSync%20Velocity) (Variables|Default|GetShouldSendLoc) (Variables|Default|GetShouldSendVel))
                (CallFunction|UpdateLocVel _vel_2 _loc_2)
                (elif (Math|Boolean|ANDBoolean (Variables|Options|GetSync%20Location) (Variables|Options|GetSync%20Rotation) (Variables|Default|GetShouldSendLoc) (Variables|Default|GetShouldSendRot))
                  (CallFunction|UpdateLocRot _loc_3 _rot_2)
                  (elif (and (Variables|Options|GetSync%20Location) (Variables|Default|GetShouldSendLoc))
                    (CallFunction|UpdateLoc (.Loc (Utilities|Rep)))
                    (elif (Math|Boolean|ANDBoolean (Variables|Options|GetSync%20Rotation) (Variables|Options|GetSync%20Velocity) (Variables|Default|GetShouldSendVel) (Variables|Default|GetShouldSendRot))
                      (CallFunction|UpdateVelRot _vel_4 _rot_3)
                      (elif (and (Variables|Options|GetSync%20Rotation) (Variables|Default|GetShouldSendRot))
                        (CallFunction|UpdateRot (.Rot (Utilities|Rep)))
                        (elif (and (Variables|Options|GetSync%20Velocity) (Variables|Default|GetShouldSendVel))
                          (CallFunction|UpdateVel (.Vel (Utilities|Rep))))))))))))))
    (else
      (goto _label))))

(fn OnRepComponentLoc
  (bind _componenttosync (Variables|Default|GetComponentToSync))
  (bind _maxerror (Variables|Options|GetMaxError))
  (if (and (> (Math|Vector|Distance(Vector) (Variables|Default|GetComponentLoc) (Transformation|GetWorldLocation (Variables|Default|GetComponentToSync))) _maxerror) (> _maxerror 0.0))
    (Transformation|SetWorldLocation _componenttosync (Variables|Default|GetComponentLoc) false true :!label _label)
    (elif (Variables|Interpolate|GetInterpolateLocation)
      (Transformation|SetWorldLocation _componenttosync (Math|Interpolation|VInterpTo (Transformation|GetWorldLocation (Variables|Default|GetComponentToSync)) (Variables|Default|GetComponentLoc) (Utilities|Time|GetWorldDeltaSeconds) (Variables|Interpolate|GetLocationInterpSpeed)) false false)
      (else
        (goto _label)))))

(fn OnRepComponentVel
  (Class|PrimitiveComponent|SetAllPhysicsLinearVelocity (Variables|Default|GetComponentToSync) (Variables|Default|GetComponentVel) false))

(fn SetUpdateFrequency
  (params (Frequency :type Integer))
  (Variables|Default|SetUpdateFrequency Frequency)
  (Class|ActorComponent|SetComponentTickInterval (/ 1.0 (Math|Conversions|ToFloat(Integer) (Variables|Default|GetUpdateFrequency)))))

(fn SetComponenttoSync
  (params (ComponentToSync :type Static%20Mesh%20Component%20Object%20Reference))
  (Variables|Default|SetComponentToSync ComponentToSync))

(fn OnRepComponentRot
  (if (Variables|Interpolate|GetInterpolate%20Rotation)
    (Transformation|SetWorldRotation (Variables|Default|GetComponentToSync) (Math|Interpolation|RInterpTo (Transformation|GetWorldRotation (Variables|Default|GetComponentToSync)) (Variables|Default|GetComponentRot) (Utilities|Time|GetWorldDeltaSeconds) (Variables|Interpolate|GetRotationInterpSpeed)) false false)
    (else
      (Transformation|SetWorldRotation (Variables|Default|GetComponentToSync) (Variables|Default|GetComponentRot) false false))))

(fn CompressRot
  (params (in :type Rotator))
  (bind (_roll _pitch _yaw) (Math|Rotator|BreakRotator in))
  (return (Math|Rotator|MakeRotator (Math|Conversions|ToFloat(Integer) (Math|Float|Truncate _roll)) (Math|Conversions|ToFloat(Integer) (Math|Float|Truncate _pitch)) (Math|Conversions|ToFloat(Integer) (Math|Float|Truncate _yaw)))))

(fn CompressVector
  (params (In :type Vector))
  (bind (_x _y _z) (Math|Vector|BreakVector In))
  (return (Math|Vector|MakeVector (Math|Conversions|ToFloat(Integer) (Math|Float|Truncate _x)) (Math|Conversions|ToFloat(Integer) (Math|Float|Truncate _y)) (Math|Conversions|ToFloat(Integer) (Math|Float|Truncate _z)))))

(fn Threashold
  (bind _rot (Utilities|Rep))
  (bind _loc (Utilities|Rep))
  (bind _vel (Utilities|Rep))
  (Utilities|FlowControl|Sequence
    (:then_0
      (if (>= (Math|Vector|Distance(Vector) _loc (Variables|Default|GetPreviousLoc)) (Variables|Options|GetPositionSendThreshold))
        (Variables|Default|SetPreviousLoc _loc)
        (Variables|Default|SetShouldSendLoc true)
        (else
          (Variables|Default|SetShouldSendLoc false))))
    (:then_1
      (if (>= (Math|Vector|Distance(Vector) _vel (Variables|Default|GetPreviousVel)) (Variables|Options|GetVelocitySendThreshold))
        (Variables|Default|SetPreviousVel _vel)
        (Variables|Default|SetShouldSendVel true)
        (else
          (Variables|Default|SetShouldSendVel false))))
    (:then_2
      (if (Math|Rotator|Equal(Rotator) _rot (Variables|Default|GetPreviousRot) (Variables|Options|GetRotationSendThreshold))
        (Variables|Default|SetPreviousRot _rot)
        (Variables|Default|SetShouldSendRot true)
        (else
          (Variables|Default|SetShouldSendRot false))))))
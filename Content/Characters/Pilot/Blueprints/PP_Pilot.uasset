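; Pilot pawn for a hovercraft with four hover springs and a machinegun added at a skeletal mesh socket on BeginPlay.
; Each tick it interpolates the HoverPlane rotation toward the aim rotation and passes it to a replication event.
; Space briefly spikes ForceToAdd, and other keys toggle spring traces and a tail component or resize the mesh.
; An overlay material flashes briefly to show damage.
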(event Custom|Rot%20Replication
  (params (NewRotation :type Rotator))
  ;[0.2016 0.2016 0.2016] Поворот корабля в точку зрения
  ;;[0 0 0] Репликация
  (Transformation|SetWorldRotation (Variables|Default|GetHoverPlane) NewRotation false true))

(event Custom|Hide%20Line%20Trace%20Serv
  (for _array_element (Utilities|Array|MakeArray (Variables|Default|GetSC_HoverSpring_Front_Left) (Variables|Default|GetSC_HoverSpring_Front_Right) (Variables|Default|GetSC_HoverSpring_Back_Right) (Variables|Default|GetSC_HoverSpring_Back_Left))
    (if (Variables|/Game/Characters/Pilot/Blueprints/SC_HoverSpring.SC_HoverSpring_C|GetShow%20Trace _array_element)
      (Variables|/Game/Characters/Pilot/Blueprints/SC_HoverSpring.SC_HoverSpring_C|SetShow%20Trace _array_element false)
      (else
        (Variables|/Game/Characters/Pilot/Blueprints/SC_HoverSpring.SC_HoverSpring_C|SetShow%20Trace _array_element true)))))

(event EventBeginPlay
  (AddComponent|AddSMCWeaponMachinegun false (Transformation|GetSocketTransform (Variables|Default|GetSkeletalMesh) "MG_1" "RTS_Actor")))

(event EventShowDamageFlickering
  (bind _skeletalmesh (Variables|Default|GetSkeletalMesh))
  (Rendering|Material|SetOverlayMaterial _skeletalmesh "/Game/Characters/VTH/MATERIALS/CUSTOM/M_Damage.M_Damage" :!class /Script/Engine.MeshComponent)
  (Utilities|FlowControl|Delay 0.1)
  (Rendering|Material|SetOverlayMaterial _skeletalmesh 0 :!class /Script/Engine.MeshComponent))

(event EventTick
  (params (DeltaSeconds :type Float%20%28single-precision%29))
  (bind _rotation (CallFunction|HoverVectoCameraVec))
  ;[0.2016 0.2016 0.2016] Поворот корабля в точку зрения
  (Transformation|SetWorldRotation (Variables|Default|GetHoverPlane) _rotation false true)
  (CallFunction|RotReplication _rotation))

(event Input|KeyboardEvents|NumPadThree
  (params (Key :type Key%20Structure :default "None")))

(event Input|KeyboardEvents|SpaceBar
  (params (Key :type Key%20Structure :default "None"))
  (:Pressed
    (Utilities|FlowControl|DoOnce false :!label _label
      (:Completed
        (Variables|Default|SetForce%20to%20Add 5e+05)
        (Utilities|FlowControl|Delay 0.01)
        (Variables|Default|SetForce%20to%20Add 6.5e+03)
        (goto _label Reset)))))

(event Input|KeyboardEvents|NumPadOne
  (params (Key :type Key%20Structure :default "None"))
  (:Pressed
    (Utilities|FlowControl|FlipFlop
      (:A
        (bind _returnvalue (AddComponent|AddSMCTail false (Transformation|GetSocketTransform (Variables|Default|GetSkeletalMesh) "Tail" "RTS_Actor")))
        (Transformation|AttachComponentToComponent _returnvalue (Variables|Default|GetSkeletalMesh) "Tail" "SnapToTarget" "SnapToTarget" "SnapToTarget" true))
      (:B
        (Components|DestroyComponent _returnvalue)))))

(event Input|KeyboardEvents|LeftCtrl
  (params (Key :type Key%20Structure :default "None"))
  (bind _skeletalmesh (Variables|Default|GetSkeletalMesh))
  (:Pressed
    (Transformation|SetWorldScale3D _skeletalmesh (- (Transformation|GetWorldScale _skeletalmesh) 0.25))))

(event Input|KeyboardEvents|NumPadSeven
  (params (Key :type Key%20Structure :default "None"))
  (:Pressed
    (for _array_element (Utilities|Array|MakeArray (Variables|Default|GetSC_HoverSpring_Front_Left) (Variables|Default|GetSC_HoverSpring_Front_Right) (Variables|Default|GetSC_HoverSpring_Back_Right) (Variables|Default|GetSC_HoverSpring_Back_Left))
      (if (Variables|/Game/Characters/Pilot/Blueprints/SC_HoverSpring.SC_HoverSpring_C|GetShow%20Trace _array_element)
        (Variables|/Game/Characters/Pilot/Blueprints/SC_HoverSpring.SC_HoverSpring_C|SetShow%20Trace _array_element false)
        (else
          (Variables|/Game/Characters/Pilot/Blueprints/SC_HoverSpring.SC_HoverSpring_C|SetShow%20Trace _array_element true))))
    (CallFunction|HideLineTraceServ)))

(event Input|KeyboardEvents|LeftAlt
  (params (Key :type Key%20Structure :default "None"))
  (bind _skeletalmesh (Variables|Default|GetSkeletalMesh))
  (:Pressed
    (Transformation|SetWorldScale3D _skeletalmesh (+ (Transformation|GetWorldScale _skeletalmesh) 0.25))))

(event Input|KeyboardEvents|NumPadTwo
  (params (Key :type Key%20Structure :default "None")))

(fn ConstructionScript)

(fn HoverVectoCameraVec
  (bind _returnvalue (Pawn|GetBaseAimRotation))
  (bind (_world_delta _interp_speed) (Utilities|FastInterp false 6.0))
  (bind _hoverplane (Variables|Default|GetHoverPlane))
  (bind _returnvalue_2 (Transformation|GetWorldRotation _hoverplane))
  (bind _returnvalue_3 (Math|Interpolation|RInterpTo _returnvalue_2 _returnvalue _world_delta _interp_speed))
  (return (Math|Rotator|MakeRotator (.roll _returnvalue_3) (.pitch _returnvalue_3) (.yaw _returnvalue_3))))

(fn OnRepRota
  (Networking|SwitchHasAuthority
    (:Authority
      (Transformation|SetWorldRotation (Variables|Default|GetHoverPlane) (Variables|Default|GetRota) false true))))
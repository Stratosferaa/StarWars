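; Test hover ship pawn that turns toward the player's aim, with debug keys for boost, tail and scale.
; Each Tick interpolates HoverPlane rotation toward base aim, clamps pitch and roll, applies it, then passes it to RotReplication.
; SpaceBar briefly spikes ForceToAdd, NumPad 1 toggles a component on the Tail socket, and LeftAlt/LeftCtrl resize the skeletal mesh.
; An Input String helper optionally prints axis values.
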(event Custom|Rot%20Replication
  (params (NewRotation :type Rotator))
  ;[0.2016 0.2016 0.2016] Поворот корабля в точку зрения
  ;;[0 0 0] Репликация
  (Transformation|SetActorRotation NewRotation))

(event EventTick
  (params (DeltaSeconds :type Float%20%28single-precision%29))
  (bind _rotation (CallFunction|HoverVectoCameraVec))
  ;[0.2016 0.2016 0.2016] Поворот корабля в точку зрения
  (Transformation|SetActorRotation _rotation true)
  (CallFunction|RotReplication _rotation))

(event Input|KeyboardEvents|NumPadThree
  (params (Key :type Key%20Structure :default "None")))

(event Input|KeyboardEvents|SpaceBar
  (params (Key :type Key%20Structure :default "None"))
  (:Pressed
    (Utilities|FlowControl|DoOnce false :!label _label
      (:Completed
        (Variables|Default|SetForce%20to%20Add 5e+05)
        (Utilities|FlowControl|Delay 0.01)
        (Variables|Default|SetForce%20to%20Add 6.5e+03)
        (goto _label Reset)))))

(event Input|KeyboardEvents|NumPadOne
  (params (Key :type Key%20Structure :default "None"))
  (:Pressed
    (Utilities|FlowControl|FlipFlop
      (:A
        (bind _returnvalue (AddComponent|AddSMCTail false (Transformation|GetSocketTransform (Variables|Default|GetSkeletalMesh) "Tail" "RTS_Actor")))
        (Transformation|AttachComponentToComponent _returnvalue (Variables|Default|GetSkeletalMesh) "Tail" "SnapToTarget" "SnapToTarget" "SnapToTarget" true))
      (:B
        (Components|DestroyComponent _returnvalue)))))

(event Input|KeyboardEvents|LeftCtrl
  (params (Key :type Key%20Structure :default "None"))
  (bind _skeletalmesh (Variables|Default|GetSkeletalMesh))
  (:Pressed
    (Transformation|SetWorldScale3D _skeletalmesh (- (Transformation|GetWorldScale _skeletalmesh) 0.25))))

(event Input|KeyboardEvents|NumPadTwo
  (params (Key :type Key%20Structure :default "None")))

(event Input|KeyboardEvents|LeftAlt
  (params (Key :type Key%20Structure :default "None"))
  (bind _skeletalmesh (Variables|Default|GetSkeletalMesh))
  (:Pressed
    (Transformation|SetWorldScale3D _skeletalmesh (+ (Transformation|GetWorldScale _skeletalmesh) 0.25))))

(fn ConstructionScript)

(fn HoverVectoCameraVec
  (bind _returnvalue (Pawn|GetBaseAimRotation))
  (bind (_world_delta _interp_speed) (Utilities|FastInterp false 6.0))
  (bind _hoverplane (Variables|Default|GetHoverPlane))
  (bind _returnvalue_2 (Transformation|GetWorldRotation _hoverplane))
  (bind _returnvalue_3 (Math|Interpolation|RInterpTo _returnvalue_2 _returnvalue _world_delta _interp_speed))
  (return (Math|Rotator|MakeRotator (Math|Float|Clamp(Float) (.roll _returnvalue_3) -25.0 25.0) (Math|Float|Clamp(Float) (.pitch _returnvalue_3) -5e+01 5e+01) (.yaw _returnvalue_3))))
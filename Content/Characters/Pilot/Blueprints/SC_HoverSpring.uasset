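; SC_HoverSpring is a hover suspension component that pushes its owner's static mesh off the surface below.
; Each Tick it traces along its negative up vector for SpringLength, with debug drawing, and on a hit applies force at its own location.
; The spring-damper force follows the hit normal, using compression and its rate of change, with higher stiffness and damping at close range.
; HoverToServ sets rotation, but its call here is disconnected.
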(event Custom|Update)

(event Custom|Hover%20To%20Serv
  (params (NewRotation :type Rotator))
  (Transformation|SetWorldRotation NewRotation false false))

(event EventBeginPlay
  ;[1 0.6916 0.1896] Warning if substep is working!
)

(event EventTick
  (params (DeltaSeconds :type Float%20%28single-precision%29))
  (Variables|Default|SetDelta%20Seconds DeltaSeconds)
  (Variables|Default|SetSpring%20Location (Transformation|GetWorldLocation))
  (bind _outhit (Collision|LineTraceByChannel (Variables|Default|GetSpring%20Location) (- (Variables|Default|GetSpring%20Location) (* (Math|Vector|GetUpVector) (Variables|Default|GetSpring%20Length))) "TraceTypeQuery1" false 0 "ForOneFrame"))
  (if (.bBlockingHit (Collision|BreakHitResult _outhit))
    (Class|PrimitiveComponent|AddForceatLocation (Actor|GetComponentbyClass (Components|GetOwner) "/Script/Engine.StaticMeshComponent") (CallFunction|CalculateSpringForce (.Distance (Collision|BreakHitResult _outhit)) (.Normal (Collision|BreakHitResult _outhit)) (.bBlockingHit (Collision|BreakHitResult _outhit))) (Variables|Default|GetSpring%20Location) "None")
    (Variables|Default|SetSuspension%20Previous (Variables|Default|GetSuspension%20Delta))))

(fn CalculateSpringForce
  (params (Distance :type Float%20%28double-precision%29) (Normal :type Vector) (Blocking%20Hit :type Boolean))
  (bind _returnvalue (< Distance 1e+02))
  (Networking|SwitchHasAuthority
    (:Authority
      _)
    (:Remote
      _))
  (Variables|Default|SetDamping (Math|Float|SelectFloat 1.2e+02 1e+01 _returnvalue))
  (Variables|Default|SetStiffness (Math|Float|SelectFloat 4e+02 2e+02 _returnvalue))
  (Variables|Default|SetSuspension%20Delta (- (Variables|Default|GetSpring%20Length) Distance))
  (return (* Normal (+ (* (Variables|Default|GetSuspension%20Delta) (Variables|Default|GetStiffness)) (* (/ (- (Variables|Default|GetSuspension%20Delta) (Variables|Default|GetSuspension%20Previous)) (Utilities|Time|GetWorldDeltaSeconds)) (Variables|Default|GetDamping))))))
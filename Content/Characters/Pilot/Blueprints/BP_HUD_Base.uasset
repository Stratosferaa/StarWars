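; Base HUD Blueprint for the pilot that creates the WBP_PilotUI widget and feeds it speed and health readouts.
; A fast looping timer, rather than Tick, samples the owning pawn's static mesh velocity.
; Displayed speed is the larger absolute forward or sideways component, scaled down and truncated to an integer, so vertical motion relative to the mesh is ignored.
; UpdateHealth passes incoming values straight through to the widget.
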(event Custom|Update%20Speed
  (bind _returnvalue (Class|HUD|GetOwningPawn))
  (bind _returnvalue_2 (Actor|GetComponentbyClass _returnvalue "/Script/Engine.StaticMeshComponent"))
  (bind _returnvalue_3 (Math|Vector|GetRightVector _returnvalue_2))
  (bind _returnvalue_4 (Transformation|GetComponentVelocity _returnvalue_2))
  (bind _returnvalue_5 (Math|Vector|GetForwardVector _returnvalue_2))
  (bind _returnvalue_6 (Math|Vector|DotProduct _returnvalue_5 _returnvalue_4))
  (bind _returnvalue_7 (Math|Vector|DotProduct _returnvalue_3 _returnvalue_4))
  (bind _returnvalue_8 (Math|Float|Absolute(Float) _returnvalue_7))
  (bind _returnvalue_9 (Math|Float|Absolute(Float) _returnvalue_6))
  (Utilities|IsValid _returnvalue
    (:Is%20Valid
      (Default|UpdateSpeed (Variables|Components|GetPilot%20UI) (Math|Float|Truncate (/ (Math|Float|SelectFloat _returnvalue_9 _returnvalue_8 (> _returnvalue_9 _returnvalue_8)) 1e+01))))))

(event EventBeginPlay
  (bind _returnvalue (UserInterface|CreateWidget "/Game/Characters/Pilot/Blueprints/WBP_PilotUI.WBP_PilotUI_C" (Variables|Default|GetPlayerOwner)))
  (bind _output_get (Variables|Components|SetPilot%20UI _returnvalue))
  (UserInterface|Viewport|AddtoPlayerScreen _output_get)
  (bind _returnvalue_2 (Utilities|Time|SetTimerbyFunctionName 0 "Update Speed" 0.05 true))
  (Variables|Default|SetUpdate%20Speed%20Timer _returnvalue_2))

(event EventUpdateHealth
  (params (Health%20Input :type Float%20%28double-precision%29))
  (Default|UpdateHealth (Variables|Components|GetPilot%20UI) Health%20Input))

(fn ConstructionScript)
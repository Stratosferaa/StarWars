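; Player controller for the arena pilot that sets up input, relays health to the HUD and adds developer debug hotkeys.
; On BeginPlay it adds the default Enhanced Input mapping context and caches the BP_HUD_Base reference.
; ForDeveloper-gated keys toggle the HUD help panel, cycle the FPS cap by console command based on measured frame rate, and toggle VSync.
; VSync debug messages are reversed relative to the value set, and ApplySettings is never called.
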(event Custom|Set%20String%20in%20Command%20Line
  (params (Command :type String))
  ;[0.04449 0.02984 0.05098] Ввод команды в консоль
  (Development|ExecuteConsoleCommand Command self))

(event EventBeginPlay
  (bind _returnvalue (PlayerController|LocalPlayerSubsystems|GetEnhancedInputLocalPlayerSubsystem))
  (Utilities|FlowControl|Sequence
    (:then_0
      ;[0.05098 0.05098 0.05098] Установка возможности отправлять запросы пешкам на движение
      (Utilities|IsValid _returnvalue
        (:Is%20Valid
          (Input|AddMappingContext _returnvalue "/Game/Characters/Pilot/Input/IMC_Default.IMC_Default" 0 "(bIgnoreAllPressedKeysUntilRelease=True,bForceImmediately=False,bNotifyUserSettings=False)"))))
    (:then_1
      ;[0.05098 0.05098 0.05098] Приведение ссылки на собственный HUD
      (bind _asbp_hud_base (Utilities|Casting|CastToBP_HUD_Base (HUD|GetHUD)))
      (Variables|Default|SetAs%20BP%20HUD%20Base%20Ref _asbp_hud_base))))

(event EventUpdateHealth
  (params (Health%20Input :type Float%20%28double-precision%29))
  ;[0.2813 0.6302 0.2423] Переброс запроса на обновление здоровья в HUD
  (Class|BPIPilotInfo|UpdateHealth(Message) (HUD|GetHUD) Health%20Input))

(event Input|KeyboardEvents|Tab
  (params (Key :type Key%20Structure :default "None"))
  (bind _as_bp_hud_base_ref (Variables|Default|GetAs%20BP%20HUD%20Base%20Ref))
  (bind _pilot_ui (Variables|/Game/Characters/Pilot/Blueprints/BP_HUD_Base.BP_HUD_Base_C|GetPilot%20UI _as_bp_hud_base_ref))
  (bind _devhelpborder (Variables|/Game/Characters/Pilot/Blueprints/WBP_PilotUI.WBP_PilotUI_C|GetDevHelpBorder _pilot_ui))
  (bind _showhelp (Variables|/Game/Characters/Pilot/Blueprints/WBP_PilotUI.WBP_PilotUI_C|GetShowHelp _pilot_ui))
  ;[0.05098 0.05098 0.05098] Вызов вспомогательного меню
  (:Pressed
    (Utilities|ForDeveloper
      (:out
        (if (Widget|IsVisible _devhelpborder)
          (Widget|SetVisibility _devhelpborder "Collapsed")
          (Widget|SetVisibility _showhelp "Visible")
          (else
            (Widget|SetVisibility _devhelpborder "Visible")
            (Widget|SetVisibility _showhelp "Collapsed")))))))

(event Input|KeyboardEvents|3
  (params (Key :type Key%20Structure :default "None"))
  (bind _returnvalue (Utilities|Time|GetWorldDeltaSeconds))
  (bind _returnvalue_2 (/ 1.0 _returnvalue))
  ;[0.05098 0.05098 0.05098] Изменение максимального FPS
  (:Pressed
    (Utilities|ForDeveloper
      (:out
        (if (Math|Float|InRange(Float) _returnvalue_2 0.0 3e+01)
          (CallFunction|SetStringinCommandLine "t.maxFPS 60")
          (Development|PrintString "Make 60" true true "(R=0.043941,G=1.000000,B=0.000000,A=1.000000)" 1e+01)
          (Development|PrintString (Utilities|String|ToString(Float) (Utilities|Time|GetWorldDeltaSeconds)) true true "(R=0.759600,G=0.786458,B=0.000000,A=1.000000)" 15.0)
          (elif (Math|Float|InRange(Float) _returnvalue_2 3e+01 6e+01)
            (CallFunction|SetStringinCommandLine "t.maxFPS 144")
            (Development|PrintString "Make 144" true true "(R=0.043941,G=1.000000,B=0.000000,A=1.000000)" 1e+01)
            (Development|PrintString (Utilities|String|ToString(Float) (Utilities|Time|GetWorldDeltaSeconds)) true true "(R=0.759600,G=0.786458,B=0.000000,A=1.000000)" 15.0)
            (elif (Math|Float|InRange(Float) _returnvalue_2 6e+01 144.0)
              (CallFunction|SetStringinCommandLine "t.maxFPS 30")
              (Development|PrintString "Make 30" true true "(R=0.043941,G=1.000000,B=0.000000,A=1.000000)" 1e+01)
              (Development|PrintString (Utilities|String|ToString(Float) (Utilities|Time|GetWorldDeltaSeconds)) true true "(R=0.759600,G=0.786458,B=0.000000,A=1.000000)" 15.0))))))))

(event Input|KeyboardEvents|4
  (params (Key :type Key%20Structure :default "None"))
  ;[0.05098 0.05098 0.05098] Включение вертикальной синхронизации
  (:Pressed
    (Utilities|ForDeveloper
      (:out
        (bind _returnvalue (Settings|GetGameUserSettings))
        (if (Class|GameUserSettings|IsVSyncEnabled _returnvalue)
          (Class|GameUserSettings|SetVSyncEnabled _returnvalue false)
          (Development|PrintString "Enabled Vsync" true true "(R=0.000000,G=1.000000,B=0.511976,A=1.000000)" 1e+01)
          (else
            (Class|GameUserSettings|SetVSyncEnabled _returnvalue true)
            (Development|PrintString "Disabled Vsync" true true "(R=1.000000,G=0.000000,B=0.000000,A=1.000000)" 1e+01)))))))

(fn ConstructionScript)
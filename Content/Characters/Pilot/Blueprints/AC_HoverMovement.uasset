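; Actor component that moves its owner's physics static mesh from Enhanced Input, judging by its name as hover movement for the pilot character.
; Move input adds acceleration-based forces along the aim yaw axes plus clamped roll torque for sideways input, while look input drives clamped controller yaw and pitch.
; Every tick, RotateReplicate re-applies the mesh's location, rotation and linear velocity, truncated to whole numbers as simple compression intended for replication.
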(event Custom|Rotate%20Replicate
  (params (SM_Component :type Static%20Mesh%20Component%20Object%20Reference) (RepLocation :type Vector) (RepRotation :type Rotator) (RepVelocity :type Vector))
  ;[0.2723 1 0.7134] Репликация
  (Transformation|SetWorldLocationAndRotation SM_Component RepLocation RepRotation false true)
  (Class|PrimitiveComponent|SetAllPhysicsLinearVelocity SM_Component RepVelocity false))

(event Input|EnhancedActionEvents|EnhancedInputActionIA_Move
  (params (ActionValue :type Vector%202D%20Structure) (ElapsedSeconds :type Float%20%28double-precision%29) (TriggeredSeconds :type Float%20%28double-precision%29) (InputAction :type Input%20Action%20Object%20Reference :default "/Game/Characters/Pilot/Input/Actions/IA_Move.IA_Move"))
  (bind _sm_component (Variables|Default|GetSM_Component))
  (bind _movement_speed (Variables|Default|GetMovement%20Speed))
  (bind (_right_left _forward_backward _torque) (CallFunction|CalculateMove (.x ActionValue) (.y ActionValue) _movement_speed))
  ;[0.2016 0.2016 0.2016] Перемещения при помощи клавиатуры
  ;;[0 0 0] Прямо 1.0 Y
  ;; Назад -1.0 Y
  ;; Влево -1.0 X
  ;; Вправо 1.0 X
  (CallFunction|Moving _sm_component _right_left _forward_backward)
  (Class|PrimitiveComponent|AddTorqueinDegrees _sm_component (CallFunction|CompressVector _torque) "None" true))

(event Input|EnhancedActionEvents|EnhancedInputActionIA_Look
  (params (ActionValue :type Vector%202D%20Structure) (ElapsedSeconds :type Float%20%28double-precision%29) (TriggeredSeconds :type Float%20%28double-precision%29) (InputAction :type Input%20Action%20Object%20Reference :default "/Game/Characters/Pilot/Input/Actions/IA_Look.IA_Look"))
  (bind _pawn_ref (Variables|Components|GetPawn%20Ref))
  ;[0.2016 0.2016 0.2016] Обзор мышкой
  ;;[0.05286 0.05286 0.05286] Right / Left
  (Pawn|Input|AddControllerYawInput _pawn_ref (Math|Float|Clamp(Float) (.x ActionValue) -1e+01 1e+01))
  ;;[0.05286 0.05286 0.05286] Up / Down
  (Pawn|Input|AddControllerPitchInput _pawn_ref (Math|Float|Clamp(Float) (.y ActionValue) -1e+01 1e+01)))

(event EventBeginPlay
  (bind _returnvalue (Components|GetOwner))
  (Variables|Components|SetPawn%20Ref (Variables|/Script/Engine.Actor|GetInstigator _returnvalue))
  (Variables|Default|SetSM_Component (Actor|GetComponentbyClass _returnvalue "/Script/Engine.StaticMeshComponent")))

(event EventTick
  (params (DeltaSeconds :type Float%20%28single-precision%29))
  (bind _sm_component (Variables|Default|GetSM_Component))
  ;[0.2723 1 0.7134] Репликация
  (CallFunction|RotateReplicate _sm_component (CallFunction|CompressVector (Transformation|GetWorldLocation _sm_component)) (CallFunction|CompressRotator (Transformation|GetWorldRotation _sm_component)) (CallFunction|CompressVector (Transformation|GetComponentVelocity _sm_component))))

(fn Moving
  (params (SM_Component :type Primitive%20Component%20Object%20Reference) (ForceLeft/Right :type Vector) (ForceFront/Back :type Vector))
  ;[0.05286 0.05286 0.05286] Вправо / Влево
  (Physics|AddForce SM_Component ForceLeft/Right "None" true)
  ;[0.05286 0.05286 0.05286] Вперёд / Назад
  (Physics|AddForce SM_Component ForceFront/Back "None" true))

(fn CalculateMove
  (params (X :type Float%20%28double-precision%29) (Y :type Float%20%28double-precision%29) (Force%20Input :type Float%20%28double-precision%29))
  (bind _pawn_ref (Variables|Components|GetPawn%20Ref))
  (bind _returnvalue (Pawn|GetBaseAimRotation _pawn_ref))
  (bind _returnvalue_2 (Math|Rotator|MakeRotator 0.0 0.0 (.yaw _returnvalue)))
  (return (* (* (Math|Vector|GetRightVector _returnvalue_2) X) Force%20Input) (* (* (Math|Vector|GetForwardVector _returnvalue_2) Y) Force%20Input) (Math|Vector|ClampVectorSize (* (* (Math|Vector|GetForwardVector _returnvalue_2) X) Force%20Input) 0.0 5e+02)))

(fn CompressVector
  (params (In :type Vector))
  (bind (_x _y _z) (Math|Vector|BreakVector In))
  (return (Math|Vector|MakeVector (Math|Conversions|ToFloat(Integer) (Math|Float|Truncate _x)) (Math|Conversions|ToFloat(Integer) (Math|Float|Truncate _y)) (Math|Conversions|ToFloat(Integer) (Math|Float|Truncate _z)))))

(fn CompressRotator
  (params (In :type Rotator))
  (bind (_roll _pitch _yaw) (Math|Rotator|BreakRotator In))
  (return (Math|Rotator|MakeRotator (Math|Conversions|ToFloat(Integer) (Math|Float|Truncate _roll)) (Math|Conversions|ToFloat(Integer) (Math|Float|Truncate _pitch)) (Math|Conversions|ToFloat(Integer) (Math|Float|Truncate _yaw)))))
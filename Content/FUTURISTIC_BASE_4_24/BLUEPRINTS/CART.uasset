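; Cart actor that rides along a referenced track's spline in the futuristic base level.
; On BeginPlay, if active, it plays a timeline at a rate set from its duration, starting from a configurable offset.
; Each update maps the timeline alpha to distance along the spline and sets the cart's world location and rotation to match.
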(event Custom|MOVECART
  (Components|Timeline|SetPlayRate (Variables|Default|GetCARTMOVER) (/ 1.0 (Variables|Default|Getduration)))
  (Components|Timeline|SetNewTime (Variables|Default|GetCARTMOVER) (Variables|Default|Getkartstartoffset))
  (bind _alpha (Timeline|CARTMOVER Play)
    (:Update
      (Variables|Default|SetALPHA _alpha)
      (Transformation|SetActorLocationAndRotation (Spline|GetLocationatDistanceAlongSpline (Variables|/Game/FUTURISTIC_BASE_4_24/BLUEPRINTS/TRACK.TRACK_C|GetUsefulSpline (Variables|Default|GetTRACKREF)) (Math|Float|Lerp 0.0 (Spline|GetSplineLength (Variables|/Game/FUTURISTIC_BASE_4_24/BLUEPRINTS/TRACK.TRACK_C|GetUsefulSpline (Variables|Default|GetTRACKREF))) (Variables|Default|GetALPHA)) "World") (Spline|GetRotationatDistanceAlongSpline (Variables|/Game/FUTURISTIC_BASE_4_24/BLUEPRINTS/TRACK.TRACK_C|GetUsefulSpline (Variables|Default|GetTRACKREF)) (Math|Float|Lerp 0.0 (Spline|GetSplineLength (Variables|/Game/FUTURISTIC_BASE_4_24/BLUEPRINTS/TRACK.TRACK_C|GetUsefulSpline (Variables|Default|GetTRACKREF))) (Variables|Default|GetALPHA)) "World")))))

(event EventBeginPlay
  (if (Variables|Default|GetACTIVECART)
    (CallFunction|MOVECART)))

(fn ConstructionScript)
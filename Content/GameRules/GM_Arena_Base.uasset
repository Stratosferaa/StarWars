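; Arena game mode that spawns and possesses a pilot pawn for each joining player.
; HandleStartingNewPlayer adds the controller to PlayerList, then spawns a PP_Pilot at the PlayerStart with the same index.
; The controller possesses the pawn and stores it as ControlledPawn on PC_Pilot_Arena, retrying after a short delay while that reference is invalid.
; PlayerRespawn and RepeateGetPawn reuse the shared last-added index rather than taking a player argument.
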(event Custom|Repeate%20Get%20Pawn
  (bind _player_pawn (Variables|Default|GetPlayer%20Pawn))
  (Pawn|Possess (Utilities|Array|Get(acopy) (Variables|Default|GetPlayer%20List) (stale EventHandleStartingNewPlayer _returnvalue)) _player_pawn)
  (bind _output_get (Variables|/Game/Characters/Pilot/Blueprints/PC_Pilot_Arena.PC_Pilot_Arena_C|SetControlled%20Pawn (.AsPC%20Pilot%20Arena (Utilities|Casting|CastToPC_Pilot_Arena (Utilities|Array|Get(acopy) (Variables|Default|GetPlayer%20List) (stale EventHandleStartingNewPlayer _returnvalue)))) _player_pawn))
  (Utilities|IsValid _output_get
    (:Is%20Not%20Valid
      (Utilities|FlowControl|Delay 0.2)
      (CallFunction|RepeateGetPawn))))

(event EventPlayerRespawn
  (bind _outactors (Actor|GetAllActorsOfClass "/Script/Engine.PlayerStart"))
  (bind _returnvalue (Game|SpawnActorfromClass "/Game/Characters/Pilot/Blueprints/PP_Pilot.PP_Pilot_C" (Transformation|GetActorTransform (Utilities|Array|Get(acopy) _outactors (stale EventHandleStartingNewPlayer _returnvalue))) "AlwaysSpawn" "MultiplyWithRoot" (Utilities|Array|Get(acopy) _outactors (stale EventHandleStartingNewPlayer _returnvalue)) 0))
  (Variables|Default|SetPlayer%20Pawn _returnvalue)
  (Pawn|Possess (Utilities|Array|Get(acopy) (Variables|Default|GetPlayer%20List) (stale EventHandleStartingNewPlayer _returnvalue)) (Variables|Default|GetPlayer%20Pawn))
  (bind _output_get (Variables|/Game/Characters/Pilot/Blueprints/PC_Pilot_Arena.PC_Pilot_Arena_C|SetControlled%20Pawn (.AsPC%20Pilot%20Arena (Utilities|Casting|CastToPC_Pilot_Arena (Utilities|Array|Get(acopy) (Variables|Default|GetPlayer%20List) (stale EventHandleStartingNewPlayer _returnvalue)))) (Variables|Default|GetPlayer%20Pawn)))
  (Utilities|IsValid _output_get
    (:Is%20Not%20Valid
      (Utilities|FlowControl|Delay 0.2)
      (CallFunction|RepeateGetPawn))))

(event EventHandleStartingNewPlayer
  (params (NewPlayer :type Player%20Controller%20Object%20Reference))
  (bind _returnvalue (Utilities|Array|Add (Variables|Default|GetPlayer%20List) NewPlayer))
  (bind _outactors (Actor|GetAllActorsOfClass "/Script/Engine.PlayerStart"))
  (bind _returnvalue_2 (Game|SpawnActorfromClass "/Game/Characters/Pilot/Blueprints/PP_Pilot.PP_Pilot_C" (Transformation|GetActorTransform (Utilities|Array|Get(acopy) _outactors _returnvalue)) "AlwaysSpawn" "MultiplyWithRoot" (Utilities|Array|Get(acopy) _outactors _returnvalue) 0))
  (Variables|Default|SetPlayer%20Pawn _returnvalue_2)
  (Pawn|Possess (Utilities|Array|Get(acopy) (Variables|Default|GetPlayer%20List) _returnvalue) (Variables|Default|GetPlayer%20Pawn))
  (bind _output_get (Variables|/Game/Characters/Pilot/Blueprints/PC_Pilot_Arena.PC_Pilot_Arena_C|SetControlled%20Pawn (.AsPC%20Pilot%20Arena (Utilities|Casting|CastToPC_Pilot_Arena (Utilities|Array|Get(acopy) (Variables|Default|GetPlayer%20List) _returnvalue))) (Variables|Default|GetPlayer%20Pawn)))
  (Utilities|IsValid _output_get
    (:Is%20Not%20Valid
      (Utilities|FlowControl|Delay 0.2)
      (CallFunction|RepeateGetPawn))))

(fn ConstructionScript)
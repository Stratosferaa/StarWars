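; BP_Machinegun_Base is a base machinegun weapon for a pilot owner, with firing currently unfinished.
; BeginPlay caches the owning BP_Pilot_Base, and left mouse input only toggles a held-trigger flag.
; Shoot, M_Shoot and S_Shoot are empty stubs.
; Disconnected logic would spawn a bullet at the Muzzle socket, push it along the pilot's forward vector, and repeat after a delay while the trigger is held.
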(event Custom|M_Shoot)

(event Custom|S_Shoot)

(event EventBeginPlay
  (bind _asbp_pilot_base (Utilities|Casting|CastToBP_Pilot_Base (Components|GetOwner)))
  (Variables|Default|SetAs%20BP%20Pilot%20Base _asbp_pilot_base))

(event Input|MouseEvents|LeftMouseButton
  (params (Key :type Key%20Structure :default "None"))
  (:Pressed
    (Variables|Default|SetShoot%20Key%20is%20Pressed true))
  (:Released
    (Variables|Default|SetShoot%20Key%20is%20Pressed false)))

(fn ConstructionScript)

(fn Shoot)
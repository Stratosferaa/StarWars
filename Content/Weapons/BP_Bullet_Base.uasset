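; Base bullet projectile actor that flies toward a given end point and damages actors it overlaps.
; StartFly plays a timeline whose updates move the bullet by constant-speed interpolation without sweeping, ignoring the passed InterpSpeed for a hard-coded value.
; Overlapping any non-owner applies fixed damage, destroys the bullet and requests damage-flicker feedback on the hit actor.
; Reaching the target also destroys it.
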(event OnComponentBeginOverlap(Bullet)
  (params (OverlappedComponent :type Primitive%20Component%20Object%20Reference) (OtherActor :type Actor%20Object%20Reference) (OtherComp :type Primitive%20Component%20Object%20Reference) (OtherBodyIndex :type Integer) (bFromSweep :type Boolean) (SweepResult :type Hit%20Result%20Structure%20%28by%20ref%29))
  (bind _returnvalue (Components|GetOwner))
  (if (!= OtherActor _returnvalue)
    (Game|Damage|ApplyDamage OtherActor 1e+01 (Game|GetInstigatorController _returnvalue) self)
    (CallFunction|DestroySelf)
    (Utilities|IsValid OtherActor
      (:Is%20Valid
        (Class|BPIDamaging|ShowDamageFlickering(Message) OtherActor)))))

(event Custom|Start%20Fly
  (params (End :type Vector) (InterpSpeed :type Float%20%28single-precision%29))
  (Utilities|IsValid self
    (:Is%20Valid
      (Timeline|Flight_TL Play
        (:Update
          (CallFunction|Flying End InterpSpeed))))))

(fn ConstructionScript)

(fn Flying
  (params (Target :type Vector) (InterpSpeed :type Float%20%28single-precision%29))
  (Transformation|SetActorLocation (Math|Interpolation|VInterptoConstant (Transformation|GetActorLocation) Target (Utilities|Time|GetWorldDeltaSeconds) 5e+03) false false)
  (if (Class|KismetMathLibrary|EqualExactlyVectorVector (Transformation|GetActorLocation) Target)
    (CallFunction|DestroySelf)))

(fn DestroySelf
  (Utilities|IsValid self
    (:Is%20Valid
      (Actor|DestroyActor))))